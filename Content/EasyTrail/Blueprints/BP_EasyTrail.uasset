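; BP_EasyTrail renders a top-down trail texture that follows player pawn 0 within a 10 m radius.
; Each tick it clears a render target and stamps gradient circles for grounded BI_EasyTrail actors and impacts queued through AddImpactPoint.
; It feeds location, movement UV offset and delta time to MPC_TrailRenderingV2.
; MM_BlendPositions then draws into RT_BlendedPositions, using these values to scroll and fade the accumulated trail.
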(event EventTick
  (params (DeltaSeconds :type Float%20%28single-precision%29))
  (bind _returnvalue (Game|Player|GetPlayerPawn 0))
  (bind _texture_render_target (Variables|Default|GetTexture%20Render%20Target))
  (bind _pawn_trail_diameter (Variables|Default|GetPawn%20Trail%20Diameter))
  (bind _returnvalue_2 (/ _pawn_trail_diameter 1e+02))
  (bind _returnvalue_3 (Math|Vector2D|MakeVector2D _returnvalue_2 _returnvalue_2))
  (bind _returnvalue_4 (* _returnvalue_3 512.0))
  (bind _returnvalue_5 (/ _returnvalue_4 2e+01))
  (Variables|Default|SetOldPosition (Variables|Default|GetCurrentPawnLocation)) ; We need previous location to offset texture
  (if (Utilities|IsValid _returnvalue)
    (bind _output_get (Variables|Default|SetCurrentPawnLocation (Transformation|GetActorLocation _returnvalue)))
    (Rendering|Material|SetVectorParameterValue "/Game/EasyTrail/Materials/MPC_TrailRenderingV2.MPC_TrailRenderingV2" "Location" (Math|Conversions|ToLinearColor(Vector) _output_get) :!class /Script/Engine.KismetMaterialLibrary)
    (Rendering|ClearRenderTarget2D _texture_render_target)
    (bind (_canvas _size _context) (Rendering|BeginDrawCanvastoRenderTarget _texture_render_target))
    (bind _outactors (Actor|GetAllActorswithInterface "/Game/EasyTrail/Blueprints/BI_EasyTrail.BI_EasyTrail_C"))
    (for _array_element _outactors
      (bind (_worldposition _ontheground) (Class|BIEasyTrail|GetActorLocationandParameters(Message) _array_element))
      (if (and _ontheground (< (Math|Vector2D|Vector2DLength (Math|Conversions|ToVector2D(Vector) (* (- _worldposition (Variables|Default|GetCurrentPawnLocation)) 0.01))) 1e+01)) ; Draw only inside 10 m radius
        (Canvas|DrawTexture :self _canvas :RenderTexture "/Game/EasyTrail/Textures/T_LinearGradient.T_LinearGradient" :ScreenPosition (+ (- (Math|Vector2D|MakeVector2D (.Y (Math|Vector2D|BreakVector2D (/ (* (Math|Conversions|ToVector2D(Vector) (* (- _worldposition (Variables|Default|GetCurrentPawnLocation)) 0.01)) 512.0) 2e+01))) (* (.X (Math|Vector2D|BreakVector2D (/ (* (Math|Conversions|ToVector2D(Vector) (* (- _worldposition (Variables|Default|GetCurrentPawnLocation)) 0.01)) 512.0) 2e+01))) -1.0)) (* _returnvalue_5 "(X=0.500000,Y=0.500000)")) "(X=256.000000,Y=256.000000)") :ScreenSize _returnvalue_5 :CoordinateSize "(X=1.000000,Y=1.000000)" :RenderColor "(R=1.000000,G=1.000000,B=0.000000,A=0.000000)" :BlendMode "BLEND_Additive" :PivotPoint "(X=0.500000,Y=0.500000)") ; Draw circles around players
      ))
    (Utilities|FlowControl|Sequence
      (:then_0
        ;[1 1 1] Draw additional Impact Points. We iterate on arrays and clear it after
        (for (_array_element_2 _array_index) (Variables|Default|GetImpactPoints)
          (if (< (Math|Vector2D|Vector2DLength (Math|Conversions|ToVector2D(Vector) (* (- _array_element_2 (Variables|Default|GetCurrentPawnLocation)) 0.01))) 1e+01)
            (Canvas|DrawTexture :self _canvas :RenderTexture "/Game/EasyTrail/Textures/T_LinearGradient.T_LinearGradient" :ScreenPosition (+ (- (Math|Vector2D|MakeVector2D (.Y (Math|Vector2D|BreakVector2D (/ (* (Math|Conversions|ToVector2D(Vector) (* (- _array_element_2 (Variables|Default|GetCurrentPawnLocation)) 0.01)) 512.0) 2e+01))) (* (.X (Math|Vector2D|BreakVector2D (/ (* (Math|Conversions|ToVector2D(Vector) (* (- _array_element_2 (Variables|Default|GetCurrentPawnLocation)) 0.01)) 512.0) 2e+01))) -1.0)) (* (/ (* (Math|Vector2D|MakeVector2D (/ (Utilities|Array|Get(acopy) (Variables|Default|GetImpactDiameter) _array_index) 1e+02) (/ (Utilities|Array|Get(acopy) (Variables|Default|GetImpactDiameter) _array_index) 1e+02)) 512.0) 2e+01) 0.5)) "(X=256.000000,Y=256.000000)") :ScreenSize (/ (* (Math|Vector2D|MakeVector2D (/ (Utilities|Array|Get(acopy) (Variables|Default|GetImpactDiameter) _array_index) 1e+02) (/ (Utilities|Array|Get(acopy) (Variables|Default|GetImpactDiameter) _array_index) 1e+02)) 512.0) 2e+01) :CoordinateSize "(X=1.000000,Y=1.000000)" :RenderColor "(R=1.000000,G=1.000000,B=0.000000,A=0.000000)" :BlendMode "BLEND_Additive" :PivotPoint "(X=0.500000,Y=0.500000)")))
        (Utilities|Array|Clear (Variables|Default|GetImpactPoints))
        (Utilities|Array|Clear (Variables|Default|GetImpactDiameter)))
      (:then_1
        (Rendering|EndDrawCanvastoRenderTarget _context)
        ;[1 1 1] Set material parameters. Used to fade out and create a trail
        (Rendering|Material|SetVectorParameterValue "/Game/EasyTrail/Materials/MPC_TrailRenderingV2.MPC_TrailRenderingV2" "PreviousPositionUV" (Math|Color|MakeColor (.Y (Math|Vector2D|BreakVector2D (/ (Math|Conversions|ToVector2D(Vector) (* (- (Variables|Default|GetCurrentPawnLocation) (Variables|Default|GetOldPosition)) 0.01)) "(X=20.000000,Y=20.000000)"))) (* (.X (Math|Vector2D|BreakVector2D (/ (Math|Conversions|ToVector2D(Vector) (* (- (Variables|Default|GetCurrentPawnLocation) (Variables|Default|GetOldPosition)) 0.01)) "(X=20.000000,Y=20.000000)"))) -1.0) 0.0) :!class /Script/Engine.KismetMaterialLibrary)
        (Rendering|Material|SetScalarParameterValue "/Game/EasyTrail/Materials/MPC_TrailRenderingV2.MPC_TrailRenderingV2" "dt" DeltaSeconds :!class /Script/Engine.KismetMaterialLibrary)
        (Rendering|DrawMaterialtoRenderTarget "/Game/EasyTrail/Textures/RT_BlendedPositions.RT_BlendedPositions" "/Game/EasyTrail/Materials/MM_BlendPositions.MM_BlendPositions") ; Draw material to render target. This will create a texture used in game
      ))))

(fn ConstructionScript)

(fn AddImpactPoint
  (params (WorldPosition :type Vector%20%28by%20ref%29) (Diameter :type Float%20%28double-precision%29%20%28by%20ref%29))
  (Utilities|Array|Add (Variables|Default|GetImpactPoints) WorldPosition)
  (Utilities|Array|Add (Variables|Default|GetImpactDiameter) Diameter))