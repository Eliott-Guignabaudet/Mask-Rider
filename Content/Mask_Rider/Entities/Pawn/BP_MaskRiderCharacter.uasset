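; Player character for Mask Rider that slides forward automatically over snowy slopes, steers sideways, performs hold-to-charge jumps and swings off branches.
; Tick tilts the mesh to the floor or velocity, sets max speed from slope and heading via a data curve, and widens FOV with speed.
; Airborne jump input arms a branch grab: a Timeline snaps to an overlapped BP_Branch, then release launches, scaled by an animation curve.
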(event OnComponentBeginOverlap(TriggerInteractionSphere)
  (params (OverlappedComponent :type Primitive%20Component%20Object%20Reference) (OtherActor :type Actor%20Object%20Reference) (OtherComp :type Primitive%20Component%20Object%20Reference) (OtherBodyIndex :type Integer) (bFromSweep :type Boolean) (SweepResult :type Hit%20Result%20Structure%20%28by%20ref%29))
  (bind _asbp_branch (Utilities|Casting|CastToBP_Branch OtherActor))
  (Variables|Default|SetCurrentBranch _asbp_branch))

(event OnComponentEndOverlap(TriggerInteractionSphere)
  (params (OverlappedComponent :type Primitive%20Component%20Object%20Reference) (OtherActor :type Actor%20Object%20Reference) (OtherComp :type Primitive%20Component%20Object%20Reference) (OtherBodyIndex :type Integer))
  (if (== OtherActor (Variables|Default|GetCurrentBranch))
    (Variables|Default|SetCurrentBranch 0)))

(event Custom|ManageAttachingBranchState
  (switch Utilities|FlowControl|Switch|SwitchonE_BranchInteraction (Variables|Default|GetCurrentBranchInteractionState)
    (:NewEnumerator1
      (Utilities|IsValid (Variables|Default|GetCurrentBranch)
        (:Is%20Valid
          (Variables|Default|SetCurrentBranchInteractionState "NewEnumerator2")
          (Development|PrintString "Attach to Branch !")
          (Variables|Default|SetStartAttachingPosition (Transformation|GetActorLocation))
          (Variables|Default|SetStartAttachingRotation (Transformation|GetActorRotation))
          (Variables|/Script/Engine.MovementComponent|SetVelocity (Variables|Character|GetCharacterMovement) "0, 0, 0")
          (bind _attachingtime (Timeline|Timeline PlayFromStart)
            (:Update
              (bind _output (Default|GetPointtoAttachTransform (Variables|Default|GetCurrentBranch)))
              (Transformation|SetActorLocation (Math|Vector|Lerp(Vector) (Variables|Default|GetStartAttachingPosition) (.location _output) _attachingtime) false false)
              (Transformation|SetActorRotation (Math|Rotator|Lerp(Rotator) (Variables|Default|GetStartAttachingRotation) (Transformation|GetSocketRotation (Variables|/Game/Mask_Rider/Entities/Branch/BP_Branch.BP_Branch_C|GetPointToAttach (Variables|Default|GetCurrentBranch)) "None") _attachingtime)))
            (:Finished
              (Variables|Default|SetCurrentBranchInteractionState "NewEnumerator3")
              (Variables|Default|SetbIsSpinning true)
              (Variables|Default|SetbIsFlying false))))))
    (:NewEnumerator3
      (Variables|/Script/Engine.MovementComponent|SetVelocity (Variables|Character|GetCharacterMovement) "0, 0, 0"))))

(event Custom|ManageSliding
  (bind _returnvalue (CallFunction|GetAngleDegreesfromFloorNormal))
  (bind _returnvalue_2 (Transformation|GetVelocity))
  (bind _returnvalue_3 (Math|Vector|VectorUp))
  (bind _returnvalue_4 (CallFunction|GetAngleBetweenUpVectorandGroundNormal))
  (bind _bisgrounded (Variables|Default|GetbIsGrounded))
  (bind _returnvalue_5 (Math|Vector|Normalize _returnvalue_2))
  (bind _returnvalue_6 (Math|Float|Absolute(Float) _returnvalue))
  (bind _returnvalue_7 (* _returnvalue_4 -1.0))
  (bind _returnvalue_8 (Math|Vector|DotProduct _returnvalue_5 _returnvalue_3))
  (bind _returnvalue_9 (Math|Float|MapRangeClamped _returnvalue_6 0.0 1.8e+02 _returnvalue_7 _returnvalue_4))
  (bind _returnvalue_10 (Class|KismetMathLibrary|DegAcos _returnvalue_8))
  (bind _returnvalue_11 (- _returnvalue_10 9e+01))
  (bind _returnvalue_12 (Math|Float|SelectFloat _returnvalue_9 _returnvalue_11 _bisgrounded))
  (Utilities|FlowControl|Sequence
    (:then_0
      (if true
        (if (.bBlockingHit (Utilities|Struct|BreakFindFloorResult (Variables|/Script/Engine.CharacterMovementComponent|GetCurrentFloor (Variables|Character|GetCharacterMovement))))
          (Pawn|Input|AddMovementInput (* (Transformation|GetActorForwardVector) (Variables|Default|GetBaseForwardInput)) 1.0 false :!label _label)
          (Development|PrintString (Utilities|String|Append "Relative roll angle " (Utilities|String|ToString(Float) _returnvalue_12)) true true "(R=0.000000,G=0.660000,B=1.000000,A=1.000000)" 2.0 "ezugrfkjazhgerfkj")
          (Transformation|SetRelativeRotation (Variables|Character|GetMesh) (Math|Rotator|MakeRotator _returnvalue_12 0.0 -9e+01) false false)
          (Development|PrintString (Utilities|String|Append "Angle between up vector and ground normal: " (Utilities|String|ToString(Float) _returnvalue_4)) true true "(R=0.000000,G=0.660000,B=1.000000,A=1.000000)" 2.0 "ghdfghfdgh"))
        (else
          (goto _label))))
    (:then_1
      (CallFunction|UpdateMaxWakSpeedbyFloorAngle)
      (Development|PrintString (Utilities|String|Append "Angle degrees from floor normal  abs" (Utilities|String|ToString(Float) (Math|Float|Absolute(Float) (CallFunction|GetAngleDegreesfromFloorNormal)))) true true "(R=0.000000,G=0.660000,B=1.000000,A=1.000000)" 2.0 "zeuiorhflkjdsfhfuiozeghrogf"))
    (:then_2
      (CallFunction|UpdateFieldOfView))))

(event Input|EnhancedActionEvents|EnhancedInputActionIA_SlideLeftRight
  (params (ActionValue :type Float%20%28double-precision%29) (ElapsedSeconds :type Float%20%28double-precision%29) (TriggeredSeconds :type Float%20%28double-precision%29) (InputAction :type Input%20Action%20Object%20Reference :default "/Game/Mask_Rider/Input/InputAction/IA_SlideLeftRight.IA_SlideLeftRight"))
  (:Triggered
    (Development|PrintString (Utilities|String|ToString(Float) ActionValue) true true "(R=0.000000,G=0.660000,B=1.000000,A=1.000000)" 2.0 "sdfgerger" :!label _label)
    (Pawn|Input|AddMovementInput (* (Transformation|GetActorRightVector) ActionValue) 1.0 false)
    (Variables|Default|SetLastSideLeftValue ActionValue))
  (:Canceled
    (goto _label))
  (:Completed
    (goto _label)))

(event Input|EnhancedActionEvents|EnhancedInputActionIA_MoveCamera
  (params (ActionValue :type Vector%202D%20Structure) (ElapsedSeconds :type Float%20%28double-precision%29) (TriggeredSeconds :type Float%20%28double-precision%29) (InputAction :type Input%20Action%20Object%20Reference :default "/Game/Mask_Rider/Input/InputAction/IA_MoveCamera.IA_MoveCamera"))
  (Transformation|AddRelativeRotation (Variables|Default|GetSpringArm) (Math|Rotator|MakeRotator 0.0 (.y ActionValue) (.x ActionValue)) false false))

(event Input|EnhancedActionEvents|EnhancedInputActionIA_Retry
  (params (ActionValue :type Boolean) (ElapsedSeconds :type Float%20%28double-precision%29) (TriggeredSeconds :type Float%20%28double-precision%29) (InputAction :type Input%20Action%20Object%20Reference :default "/Game/Mask_Rider/Input/InputAction/IA_Retry.IA_Retry"))
  (bind _returnvalue (Game|GetCurrentLevelName true))
  (Game|OpenLevel(byName) (Utilities|String|StringToName _returnvalue)))

(event Input|EnhancedActionEvents|EnhancedInputActionIA_Jump
  (params (ActionValue :type Boolean) (ElapsedSeconds :type Float%20%28double-precision%29) (TriggeredSeconds :type Float%20%28double-precision%29) (InputAction :type Input%20Action%20Object%20Reference :default "/Game/Mask_Rider/Input/InputAction/IA_Jump.IA_Jump"))
  (:Triggered
    (if (Variables|Default|GetbIsGrounded)
      (if (Variables|Default|GetbIsCharging)
        _
        (else
          (CallFunction|StartCharging ElapsedSeconds)))
      (CallFunction|UpdateChargingTime ElapsedSeconds)
      (elif (Utilities|Enum|Equal(Enum) (Variables|Default|GetCurrentBranchInteractionState) "NewEnumerator0")
        (Variables|Default|SetCurrentBranchInteractionState "NewEnumerator1"))))
  (:Started
    (if (Variables|Default|GetbIsGrounded)
      (CallFunction|StartCharging ElapsedSeconds)))
  (:Completed
    (Utilities|FlowControl|Sequence
      (:then_0
        (if (Variables|Default|GetbIsCharging)
          (CallFunction|PerformJump ElapsedSeconds)))
      (:then_1
        (if (Utilities|Enum|Equal(Enum) (Variables|Default|GetCurrentBranchInteractionState) "NewEnumerator3")
          (Variables|Default|SetCurrentBranchInteractionState "NewEnumerator0")
          (Variables|Default|SetbIsSpinning false)
          (Character|LaunchCharacter (* (Math|Vector|GetForwardVector (Variables|/Game/Mask_Rider/Entities/Branch/BP_Branch.BP_Branch_C|GetPointToAttach (Variables|Default|GetCurrentBranch))) (* (Math|Float|MakeLiteralFloat (Variables|/Game/Mask_Rider/Entities/Pawn/Data/PDA_PlayerData.PDA_PlayerData_C|GetBranchLaunchPower (Variables|Default|GetPlayerData))) (Math|Float|Clamp(Float) (Animation|Curves|GetCurveValue (Components|SkeletalMesh|GetAnimInstance (Variables|Character|GetMesh)) "LaunchPowerFactor") 0.3))) false false))))))

(event EventBeginPlay
  (Variables|Default|SetbIsGrounded true)
  (Audio|Components|Audio|Stop (Variables|Default|GetCharchingForceFeedback))
  (Variables|Default|SetCurrentBranchInteractionState "NewEnumerator0")
  (Variables|/Script/Engine.CharacterMovementComponent|SetBrakingDecelerationWalking (Variables|Character|GetCharacterMovement) (Variables|/Game/Mask_Rider/Entities/Pawn/Data/PDA_PlayerData.PDA_PlayerData_C|GetBrakingDecelerationSpeed (Variables|Default|GetPlayerData)))
  (Niagara|SpawnSystemAttached "/Game/Mask_Rider/Art/VFX/NS_SnowCubes.NS_SnowCubes" (Variables|Character|GetMesh) "None" "0, 0, 0" "0, 0, 0" "KeepRelativeOffset" false))

(event Collision|EventActorBeginOverlap
  (params (OtherActor :type Actor%20Object%20Reference)))

(event EventTick
  (params (DeltaSeconds :type Float%20%28single-precision%29))
  (bind _playerdata (Variables|Default|GetPlayerData))
  (bind _currentlandingparticle (Variables|Default|GetCurrentLandingParticle))
  (if (Utilities|Enum|Equal(Enum) (Variables|Default|GetCurrentBranchInteractionState) "NewEnumerator0")
    (CallFunction|ManageSliding)
    (bind _output_get (Variables|Default|SetbIsGrounded (and (.bBlockingHit (Utilities|Struct|BreakFindFloorResult (Variables|/Script/Engine.CharacterMovementComponent|GetCurrentFloor (Variables|Character|GetCharacterMovement)))) (not (Variables|Default|GetbIsSpinning)))))
    (Variables|Default|SetbIsFlying (not _output_get))
    (Variables|/Script/Engine.CharacterMovementComponent|SetRotationRate (Variables|Character|GetCharacterMovement) (Math|Rotator|SelectRotator (Math|Rotator|MakeRotator 0.0 0.0 (Math|Float|MapRangeClamped (Variables|Default|GetCurrentSpeed) 0.0 2e+03 (Variables|/Game/Mask_Rider/Entities/Pawn/Data/PDA_PlayerData.PDA_PlayerData_C|GetMaxRotationSpeedSliding _playerdata) (Variables|/Game/Mask_Rider/Entities/Pawn/Data/PDA_PlayerData.PDA_PlayerData_C|GetMinRotationSpeedSliding _playerdata))) (Math|Rotator|MakeRotator 0.0 0.0 (Variables|/Game/Mask_Rider/Entities/Pawn/Data/PDA_PlayerData.PDA_PlayerData_C|GetRotationSpeedFlying (Variables|Default|GetPlayerData))) (Variables|Default|GetbIsGrounded)))
    (Variables|Default|SetCurrentSpeed (Math|Vector|VectorLength (Transformation|GetVelocity)))
    (Utilities|IsValid _currentlandingparticle
      (:Is%20Valid
        (Transformation|SetWorldLocation _currentlandingparticle (Transformation|GetActorLocation) false false)))
    (else
      (CallFunction|ManageAttachingBranchState))))

(event Collision|EventHit
  (params (MyComp :type Primitive%20Component%20Object%20Reference) (Other :type Actor%20Object%20Reference) (OtherComp :type Primitive%20Component%20Object%20Reference) (bSelfMoved :type Boolean) (HitLocation :type Vector :default "0, 0, 0") (HitNormal :type Vector :default "0, 0, 0") (NormalImpulse :type Vector :default "0, 0, 0") (Hit :type Hit%20Result%20Structure%20%28by%20ref%29))
  (Variables|Default|SetbIsFlying false)
  (if (and (Utilities|Enum|NotEqual(Enum) (Variables|Default|GetCurrentBranchInteractionState) "NewEnumerator2") (Utilities|Enum|NotEqual(Enum) (Variables|Default|GetCurrentBranchInteractionState) "NewEnumerator3"))
    (Audio|Components|Audio|Play (Variables|Default|GetLandingForceFeedback) 0.0)
    (Variables|Default|SetCurrentBranchInteractionState "NewEnumerator0")
    (Components|Activation|Deactivate (Variables|Default|GetNS_JumpRibbon))
    (bind _returnvalue (Niagara|SpawnSystemAttached "/Game/Mask_Rider/Art/VFX/NS_Landing.NS_Landing" (Variables|Character|GetMesh) "None" "0, 0, 0" "0, 0, 0" "KeepRelativeOffset" true true "AutoRelease"))
    (Variables|Default|SetCurrentLandingParticle _returnvalue)))

(fn ConstructionScript)

(fn GetAngleDegreesfromFloorNormal
  (bind _returnvalue (Transformation|GetActorForwardVector))
  (bind _charactermovement (Variables|Character|GetCharacterMovement))
  (bind _returnvalue_2 (Math|Vector2D|MakeVector2D (.x _returnvalue) (.y _returnvalue)))
  (bind _currentfloor (Variables|/Script/Engine.CharacterMovementComponent|GetCurrentFloor _charactermovement))
  (bind _hitresult (Utilities|Struct|BreakFindFloorResult _currentfloor))
  (bind (_x _y) (Math|Vector2D|BreakVector2D _returnvalue_2))
  (bind (_x_2 _y_2) (Math|Vector2D|BreakVector2D _returnvalue_2))
  (bind (_bblockinghit _binitialoverlap _time _distance _location _impactpoint _normal _impactnormal) (Collision|BreakHitResult _hitresult))
  (bind _returnvalue_3 (Math|Vector|RotateVectorAroundAxis _impactnormal 9e+01 "0.000000,0.000000,1.000000"))
  (bind (_x_3 _y_3) (Math|Vector|BreakVector _returnvalue_3))
  (bind _returnvalue_4 (Math|Vector2D|MakeVector2D _x_3 _y_3))
  (bind (_x_4 _y_4) (Math|Vector2D|BreakVector2D _returnvalue_4))
  (bind (_x_5 _y_5) (Math|Vector2D|BreakVector2D _returnvalue_4))
  (Rendering|Debug|DrawDebugLine _location (+ _location (* _normal (Math|Float|MakeLiteralFloat 1e+02))) "(R=1.000000,G=0.018913,B=0.000000,A=1.000000)" 1e+01 0.0)
  (return (Class|KismetMathLibrary|DegAtan2 (+ (* _x_5 _x_2) (* _y_5 _y_2)) (- (* _x_4 _y) (* _y_4 _x)))))

(fn UpdateMaxWakSpeedbyFloorAngle
  (bind _returnvalue (CallFunction|GetAngleDegreesfromFloorNormal))
  (bind _returnvalue_2 (CallFunction|GetAngleBetweenUpVectorandGroundNormal))
  (bind _playerdata (Variables|Default|GetPlayerData))
  (bind _playerdata_2 (Variables|Default|GetPlayerData))
  (bind _returnvalue_3 (Math|Float|Absolute(Float) _returnvalue))
  (bind _returnvalue_4 (Math|Float|MapRangeClamped _returnvalue_2 0.0 8e+01 0.0 1.0))
  (bind _speedmultiplier (Variables|/Game/Mask_Rider/Entities/Pawn/Data/PDA_PlayerData.PDA_PlayerData_C|GetSpeedMultiplier _playerdata_2))
  (bind _speedfactorbyangle (Variables|/Game/Mask_Rider/Entities/Pawn/Data/PDA_PlayerData.PDA_PlayerData_C|GetSpeedFactorByAngle _playerdata))
  (bind _returnvalue_5 (Math|Curves|GetFloatValue _speedfactorbyangle _returnvalue_4))
  (bind _returnvalue_6 (- _returnvalue_3 9e+01))
  (bind _returnvalue_7 (* _returnvalue_6 _speedmultiplier))
  (bind _returnvalue_8 (* _returnvalue_7 _returnvalue_5))
  (bind _output_get (Variables|/Script/Engine.CharacterMovementComponent|SetMaxWalkSpeed (Variables|Character|GetCharacterMovement) (Math|Float|SelectFloat (Math|Float|Clamp(Float) _returnvalue_8 (Variables|/Game/Mask_Rider/Entities/Pawn/Data/PDA_PlayerData.PDA_PlayerData_C|GetMinSpeed (Variables|Default|GetPlayerData)) _returnvalue_8) (Variables|/Game/Mask_Rider/Entities/Pawn/Data/PDA_PlayerData.PDA_PlayerData_C|GetMinSpeed (Variables|Default|GetPlayerData)) (> _returnvalue_3 9e+01))))
  (Development|PrintString (Utilities|String|Append "Current Max Walk speed: " (Utilities|String|ToString(Float) _output_get)) true true "(R=1.000000,G=0.856640,B=0.000000,A=1.000000)" 2.0 "iorehkgfhdklfhjg"))

(fn PerformJump
  (params (InputPin :type Float%20%28double-precision%29))
  (Variables|/Script/Engine.CharacterMovementComponent|SetJumpZVelocity (Variables|Character|GetCharacterMovement) (* (Math|Float|Clamp(Float) (- InputPin (Variables|Default|GetStartChargingTime)) 0.1 (Variables|Default|GetMaxChargingTime)) (Variables|/Game/Mask_Rider/Entities/Pawn/Data/PDA_PlayerData.PDA_PlayerData_C|GetJumpForce (Variables|Default|GetPlayerData))))
  (Character|Jump)
  (Variables|Default|SetbIsGrounded false)
  (Variables|Default|SetbIsFlying true)
  (Variables|Default|SetbIsCharging false)
  (Audio|Components|Audio|Stop (Variables|Default|GetCharchingForceFeedback))
  (Components|Activation|Activate (Variables|Default|GetNS_JumpRibbon) false))

(fn StartCharging
  (params (InputPin :type Float%20%28double-precision%29))
  (Variables|Default|SetStartChargingTime InputPin)
  (Variables|Default|SetbIsCharging true)
  (Audio|Components|Audio|Play (Variables|Default|GetCharchingForceFeedback) 0.0)
  (return))

(fn UpdateChargingTime
  (params (A :type Float%20%28double-precision%29))
  (bind _output_get (Variables|Default|SetChargingTime (- A (Variables|Default|GetStartChargingTime))))
  (Variables|/Script/Engine.ForceFeedbackComponent|SetIntensityMultiplier (Variables|Default|GetCharchingForceFeedback) (/ (Math|Float|Clamp(Float) _output_get 0.0 (Variables|Default|GetMaxChargingTime)) 2.0)))

(fn UpdateFieldOfView
  (Camera|SetFieldOfView (Variables|Default|GetCamera) (Math|Float|Lerp (Variables|/Script/Engine.CameraComponent|GetFieldOfView (Variables|Default|GetCamera)) (Math|Float|MapRangeClamped (Math|Vector|VectorLength (Transformation|GetVelocity)) 5e+02 2.5e+03 (select (Variables|Default|GetbIsCharging) (Math|Float|MapRangeClamped (Variables|Default|GetChargingTime) 0.0 (Variables|Default|GetMaxChargingTime) 8e+01 7e+01) 8e+01) (select (Variables|Default|GetbIsCharging) (Math|Float|MapRangeClamped (Variables|Default|GetChargingTime) 0.0 (Variables|Default|GetMaxChargingTime) 1.2e+02 1e+02) 1.2e+02)) (* (Utilities|Time|GetWorldDeltaSeconds) 5.0))))

(fn GetAngleBetweenUpVectorandGroundNormal
  (return (Class|KismetMathLibrary|DegAcos (Math|Vector|DotProduct (Math|Vector|Normalize (Transformation|GetActorUpVector)) (Math|Vector|Normalize (.Normal (Collision|BreakHitResult (.HitResult (Utilities|Struct|BreakFindFloorResult (Variables|/Script/Engine.CharacterMovementComponent|GetCurrentFloor (Variables|Character|GetCharacterMovement)))))))))))

(fn GetActorLocationandParameters
  (return (Transformation|GetActorLocation) (AI|Components|NavMovement|IsMovingonGround (Variables|Character|GetCharacterMovement))))