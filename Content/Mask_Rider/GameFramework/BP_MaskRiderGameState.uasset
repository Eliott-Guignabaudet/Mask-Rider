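; Game state for Mask Rider that tracks a match countdown timer.
; On BeginPlay it reads the starting duration from BP_MaskRiderGameMode and calls StartTimer, which sets the running flag and reloads that duration.
; Tick subtracts delta time from CurrentTimer while running, with no clamp or expiry handling in this Blueprint.
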(event EventBeginPlay
  (Variables|Default|SetbIsTimerStarted false)
  (bind _asbp_mask_rider_game_mode (Utilities|Casting|CastToBP_MaskRiderGameMode (Game|GetGameMode)))
  (Variables|Default|SetCurrentTimer (Variables|/Game/Mask_Rider/GameFramework/BP_MaskRiderGameMode.BP_MaskRiderGameMode_C|GetTimer _asbp_mask_rider_game_mode))
  (CallFunction|StartTimer))

(event EventTick
  (params (DeltaSeconds :type Float%20%28single-precision%29))
  (if (Variables|Default|GetbIsTimerStarted)
    (Variables|Default|SetCurrentTimer (- (Variables|Default|GetCurrentTimer) DeltaSeconds))))

(fn ConstructionScript)

(fn StartTimer
  (bind _asbp_mask_rider_game_mode (Utilities|Casting|CastToBP_MaskRiderGameMode (Game|GetGameMode)))
  (Variables|Default|SetbIsTimerStarted true)
  (Variables|Default|SetCurrentTimer (Variables|/Game/Mask_Rider/GameFramework/BP_MaskRiderGameMode.BP_MaskRiderGameMode_C|GetTimer _asbp_mask_rider_game_mode)))